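; Actor that links left and right hand follower actors, likely hand triggers, to the VR pawn's motion controllers.
; While its pawn reference is unset, Tick waits briefly, then finds the VRPawnCustom_Bp in the level and assigns the hands.
; A Set Follower Target helper writes each motion controller into the follower's Follow_Motion_Ctrl_Cmp_Bp component as its target.
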(event `self.ReceiveBeginPlay`)

(event `self.ReceiveTick`
  (params (DeltaSeconds :type "Float (single-precision)"))
  (if (== (`self.VR Pawn`) null)
    (`KismetSystemLibrary.Delay` 0.2)
    (bind _returnvalue (`GameplayStatics.GetActorOfClass` "/Game/VRPawnCustom_Bp.VRPawnCustom_Bp_C"))
    (bind _output_get (set `self.VR Pawn` _returnvalue))
    (`self.Assign Hands Fc` _output_get)))

(fn `Assign Hands Fc`
  (params (VrPawnParam :type "/Game/VRPawnCustom_Bp Object Reference"))
  (`self.Set Follower Target` (`self.Left Hand Follower`) (`/Game/VRPawnCustom_Bp.MotionControllerLeft` VrPawnParam)
    (:`Out`
      (`self.Set Follower Target` (`self.Right Hand Follower`) (`/Game/VRPawnCustom_Bp.MotionControllerRight` VrPawnParam)))))

(fn `UserConstructionScript`)